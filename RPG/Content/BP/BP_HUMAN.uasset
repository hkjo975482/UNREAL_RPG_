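; Player human character that moves, sprints, fights zombies (BP_殭屍) and collects keys, with a HUD widget created at BeginPlay.
; A weapon toggle reattaches the weapon between hand and leg sockets; light and heavy attacks alternate two montages using DoOnce gates and delayed counter resets.
; Weapon and right-foot overlaps damage zombies, with functions toggling movement and weapon overlaps.
; 受傷 subtracts health and sets the death flag, which Tick turns into a frozen death animation.
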(event OnComponentBeginOverlap(武器碰撞區域)
  (params (OverlappedComponent :type Primitive%20Component%20Object%20Reference) (OtherActor :type Actor%20Object%20Reference) (OtherComp :type Primitive%20Component%20Object%20Reference) (OtherBodyIndex :type Integer) (bFromSweep :type Boolean) (SweepResult :type Hit%20Result%20Structure%20%28by%20ref%29))
  (bind _asbp_殭屍 (Utilities|Casting|CastToBP_殭屍 OtherActor))
  (Default|受傷 _asbp_殭屍 3e+01))

(event OnComponentBeginOverlap(CapsuleComponent)
  (params (OverlappedComponent :type Primitive%20Component%20Object%20Reference) (OtherActor :type Actor%20Object%20Reference) (OtherComp :type Primitive%20Component%20Object%20Reference) (OtherBodyIndex :type Integer) (bFromSweep :type Boolean) (SweepResult :type Hit%20Result%20Structure%20%28by%20ref%29))
  (bind _喇叭 (Variables|Default|Get喇叭))
  (bind _asbp_鑰匙 (Utilities|Casting|CastToBP_鑰匙 OtherActor))
  (bind _asbp_鑰匙_2 (Utilities|Casting|CastToBP_鑰匙 _asbp_鑰匙))
  (Audio|Components|Audio|SetSound _喇叭 "/Game/音效/鑰匙音效.鑰匙音效")
  (Audio|Components|Audio|Play _喇叭 0.0)
  (Actor|DestroyActor _asbp_鑰匙_2)
  (Math|Integer|IncrementInt (Variables|Default|Get鑰匙數量)))

(event OnComponentBeginOverlap(右腳直攻)
  (params (OverlappedComponent :type Primitive%20Component%20Object%20Reference) (OtherActor :type Actor%20Object%20Reference) (OtherComp :type Primitive%20Component%20Object%20Reference) (OtherBodyIndex :type Integer) (bFromSweep :type Boolean) (SweepResult :type Hit%20Result%20Structure%20%28by%20ref%29))
  (bind _asbp_殭屍 (Utilities|Casting|CastToBP_殭屍 OtherActor))
  (Default|受傷 _asbp_殭屍 4e+01))

(event EventBeginPlay
  ;[1 1 1] Comment
  (bind _returnvalue (UserInterface|CreateWidget "/Game/BP/BW_介面.BW_介面_C" (Game|GetPlayerController 0)))
  (UserInterface|Viewport|AddtoViewport _returnvalue 0))

(event EventTick
  (params (DeltaSeconds :type Float%20%28single-precision%29))
  (if (Variables|Default|Get是否死亡)
    (Utilities|FlowControl|DoOnce false
      (:Completed
        (Components|Animation|PlayAnimation (Variables|Character|GetMesh) "/Game/動作/主角死亡_Montage.主角死亡_Montage" false)
        (Utilities|FlowControl|Delay 2.0)
        (Components|Timeline|SetPlayRate (Variables|Character|GetMesh) 0.0)))))

(event Input|ActionEvents|InputAction衝刺
  (params (Key :type Key%20Structure :default "None"))
  (bind _charactermovement (Variables|Character|GetCharacterMovement))
  ;[1 1 1] Comment
  (:Pressed
    (Variables|/Script/Engine.CharacterMovementComponent|SetMaxWalkSpeed _charactermovement 1.2e+03))
  (:Released
    (Variables|/Script/Engine.CharacterMovementComponent|SetMaxWalkSpeed _charactermovement 6e+02)))

(event Input|ActionEvents|InputAction武器
  (params (Key :type Key%20Structure :default "None"))
  (bind _weapon (Variables|Default|Getweapon))
  ;[1 1 1] 切換武器
  (:Pressed
    (if (not (Variables|Default|Get是否死亡))
      (Variables|Default|Set拿武器 (not (Variables|Default|Get拿武器)))
      (Animation|Montage|PlayMontage (Variables|Character|GetMesh) "/Game/動作/拔武器_Montage.拔武器_Montage"
        (:then
          (if (Variables|Default|Get拿武器)
            (Utilities|FlowControl|Delay 0.5)
            (Transformation|AttachComponentToComponent _weapon (Variables|Default|Get右手) "None" "KeepRelative" "KeepRelative" "KeepRelative" true)
            (else
              (Utilities|FlowControl|Delay 0.5)
              (Transformation|AttachComponentToComponent _weapon (Variables|Default|Get右腳) "None" "KeepRelative" "KeepRelative" "KeepRelative" true)))
          (Components|MoveComponentTo 0 "0, 0, 0" "0, 0, 0" false false 0.2 false))))))

(event Input|ActionEvents|InputAction第一段攻擊
  (params (Key :type Key%20Structure :default "None"))
  ;[1 1 1] Comment
  (:Pressed
    (if (not (Variables|Default|Get是否死亡))
      (Utilities|FlowControl|DoOnce false :!label _label
        (:Completed
          (if (Variables|Default|Get拿武器)
            (Animation|Montage|PlayMontage (Variables|Character|GetMesh) (Utilities|Select :Index (Math|Integer|%(Integer) (Variables|Default|Get第一段攻擊次數) 2) :Option%200 "/Game/動作/攻擊第一段_Montage.攻擊第一段_Montage" :Option%201 "/Game/動作/攻擊第二段_Montage.攻擊第二段_Montage") 1.7
              (:then
                (bind _result (Math|Integer|IncrementInt (Variables|Default|Get第一段攻擊次數))
                  (:%20%20
                    (Development|PrintString (Utilities|String|ToString(Integer) _result))
                    (Utilities|FlowControl|Delay 0.4)
                    (Utilities|FlowControl|Sequence
                      (:then_0
                        (goto _label Reset))
                      (:then_1
                        (Utilities|FlowControl|Delay 0.85)
                        (Variables|Default|Set第一段攻擊次數 0)))))))
            (else
              (goto _label Reset))))))))

(event Input|ActionEvents|InputAction重擊
  (params (Key :type Key%20Structure :default "None"))
  ;[1 1 1] 重擊
  (:Pressed
    (if (not (Variables|Default|Get是否死亡))
      (if (Variables|Default|Get拿武器)
        (Utilities|FlowControl|DoOnce false :!label _label
          (:Completed
            (Animation|Montage|PlayMontage (Variables|Character|GetMesh) (Utilities|Select :Index (Math|Integer|%(Integer) (Variables|Default|Get重擊) 2) :Option%200 "/Game/動作/重擊第一段_Montage.重擊第一段_Montage" :Option%201 "/Game/動作/重擊第二段_Montage.重擊第二段_Montage") 1.7
              (:then
                (bind _result (Math|Integer|IncrementInt (Variables|Default|Get重擊))
                  (:%20%20
                    (Development|PrintString (Utilities|String|ToString(Integer) _result))
                    (Utilities|FlowControl|Delay 0.5)
                    (Utilities|FlowControl|Sequence
                      (:then_0
                        (goto _label Reset))
                      (:then_1
                        (Utilities|FlowControl|Delay 0.85)
                        (Variables|Default|Set重擊 0)))))))))))))

(event Input|AxisEvents|InputAxisLookUp
  (params (AxisValue :type Float%20%28single-precision%29))
  ;[1 1 1] 滑鼠輸入
  (Pawn|Input|AddControllerPitchInput AxisValue))

(event Input|AxisEvents|InputAxisTurn
  (params (AxisValue :type Float%20%28single-precision%29))
  ;[1 1 1] 滑鼠輸入
  (Pawn|Input|AddControllerYawInput AxisValue))

(event Input|AxisEvents|InputAxisMoveForward
  (params (AxisValue :type Float%20%28single-precision%29))
  ;[1 1 1] 動作
  (if (not (Variables|Default|Get是否死亡))
    (if (Variables|Default|Get是否移動)
      (Pawn|Input|AddMovementInput (Math|Vector|GetForwardVector (Math|Rotator|MakeRotator 0.0 0.0 (.Yaw (Math|Rotator|BreakRotator (Pawn|GetControlRotation :!class /Script/Engine.Pawn))))) AxisValue false))))

(event Input|AxisEvents|InputAxisMoveRight
  (params (AxisValue :type Float%20%28single-precision%29))
  ;[1 1 1] 動作
  (if (not (Variables|Default|Get是否死亡))
    (if (Variables|Default|Get是否移動)
      (Pawn|Input|AddMovementInput (Math|Vector|GetRightVector (Math|Rotator|MakeRotator 0.0 0.0 (.Yaw (Math|Rotator|BreakRotator (Pawn|GetControlRotation :!class /Script/Engine.Pawn))))) AxisValue false))))

(fn ConstructionScript)

(fn 切換移動
  (params (是否移動 :type Boolean))
  (Variables|Default|Set是否移動 是否移動))

(fn 切換武器碰撞區域
  (params (是否顯示武器碰撞區域 :type Boolean))
  (Variables|/Script/Engine.PrimitiveComponent|SetbGenerateOverlapEvents (Variables|Default|Get武器碰撞區域) 是否顯示武器碰撞區域))

(fn 受傷
  (params (傷害值 :type Float%20%28single-precision%29))
  (if (not (Variables|Default|Get是否死亡))
    (Variables|Default|Set血量 (- (Variables|Default|Get血量) 傷害值))
    (Animation|PlayAnimMontage self "/Game/動作/主角被打_Montage.主角被打_Montage" 1.0 "None")
    (if (<= (Variables|Default|Get血量) 0.0)
      (Variables|Default|Set是否死亡 true))))