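; Zombie AI pawn that wanders, chases humans it sees, plays an attack animation and can be killed.
; BeginPlay starts a loop of random nearby moves with random pauses while it has no target.
; Its sensor's OnSeePawn targets BP_HUMAN, moves to it and plays a DoOnce-gated attack montage, then resumes wandering.
; 受傷 subtracts health and plays hit or death montages, while Tick flags death and destroys the actor after a delay.
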(event OnSeePawn(感受器)
  (params (Pawn :type Pawn%20Object%20Reference))
  ;[1 1 1] Comment
  (if (not (Variables|Default|Get攻擊玩家))
    (bind _asbp_human (Utilities|Casting|CastToBP_HUMAN Pawn))
    (bind _output_get (Variables|Default|Set人物物件 _asbp_human))
    (AI|AIMoveTo self "0, 0, 0" _output_get 5.0 false
      (:OnSuccess
        (Utilities|FlowControl|DoOnce false :!label _label
          (:Completed
            (Animation|Montage|PlayMontage (Variables|Character|GetMesh) "/Game/殭屍動畫/殭屍攻擊_Montage.殭屍攻擊_Montage" 1.2
              (:then
                (Variables|Default|Set攻擊玩家 true)
                (Variables|Default|Set人物物件 0))
              (:OnCompleted
                (Variables|Default|Set攻擊玩家 false)
                (Utilities|FlowControl|Delay 0.3)
                (Utilities|FlowControl|Sequence
                  (:then_0
                    (goto _label Reset))
                  (:then_1
                    ;[1 1 1] 隨機走動
                    (if (not (Variables|Default|Get攻擊玩家)) :!label _label_2
                      (Utilities|IsValid (Variables|Default|Get人物物件)
                        (:Is%20Not%20Valid
                          (AI|AIMoveTo self (.RandomLocation (AI|Navigation|GetRandomReachablePointinRadius (Transformation|GetWorldLocation (Variables|Character|GetMesh)) 5e+02 0 0)) 0 5.0 false
                            (:OnSuccess
                              (Utilities|FlowControl|Sequence
                                (:then_0
                                  _)))
                            (:OnFail
                              _))
                          (Utilities|FlowControl|Delay (Math|Random|RandomFloatinRange 1.0 3.0))
                          (goto _label_2))))))))))))))

(event EventTick
  (params (DeltaSeconds :type Float%20%28single-precision%29))
  (if (<= (Variables|Default|Get血量) 0.0)
    (Variables|Default|Set是否死亡 true)
    (Utilities|FlowControl|DoOnce false
      (:Completed
        (Utilities|FlowControl|Delay 2.6)
        (Actor|DestroyActor self)))))

(event EventBeginPlay
  ;[1 1 1] 隨機走動
  (Utilities|IsValid (Variables|Default|Get人物物件) :!label _label
    (:Is%20Not%20Valid
      (AI|AIMoveTo self (.RandomLocation (AI|Navigation|GetRandomReachablePointinRadius (Transformation|GetWorldLocation (Variables|Character|GetMesh)) 5e+02 0 0)) 0 5.0 false
        (:OnSuccess
          (Utilities|FlowControl|Sequence
            (:then_0
              _)))
        (:OnFail
          _))
      (Utilities|FlowControl|Delay (Math|Random|RandomFloatinRange 1.0 3.0))
      (if (not (Variables|Default|Get攻擊玩家))
        (goto _label)))))

(fn ConstructionScript)

(fn 受傷
  (params (傷害值 :type Float%20%28single-precision%29))
  (if (not (Variables|Default|Get是否死亡))
    (Variables|Default|Set血量 (- (Variables|Default|Get血量) 傷害值))
    (Animation|PlayAnimMontage self "/Game/殭屍動畫/殭屍被打_Montage.殭屍被打_Montage" 1.0 "None")
    (if (<= (Variables|Default|Get血量) 0.0)
      (Animation|PlayAnimMontage self "/Game/殭屍動畫/殭屍死掉_Montage.殭屍死掉_Montage" 1.0 "None"))))